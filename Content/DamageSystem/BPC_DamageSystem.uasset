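; BPC_DamageSystem is a damage component that tracks Health and a death flag through Heal and TakeDamage functions.
; TakeDamage subtracts the damage struct's amount and returns true while alive, but sets IsDead on any hit because its health check is unwired.
; Heal returns current Health unchanged, as the clamped addition never runs.
; The DamageResponse switch is also disconnected, and BeginPlay and Tick are empty.
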(event EventBeginPlay)

(event EventTick
  (params (DeltaSeconds :type Float%20%28single-precision%29)))

(fn Heal
  (params (Amount :type Float%20%28double-precision%29))
  (if (not (Variables|Default|GetIsDead))
    (return (stale _output_get))))

(fn TakeDamage
  (params (DamageInfo :type S%20Damage%20Info%20Structure))
  (if (not (Variables|Default|GetIsDead))
    (bind _output_get (Variables|Default|SetHealth (- (Variables|Default|GetHealth) (.Amount (Utilities|Struct|BreakS_DamageInfo DamageInfo)))))
    (if true
      (Variables|Default|SetIsDead true))
    (return true)))